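; Boss enemy character that equips its weapon mesh on the hand socket and runs a two-phase fight.
; BossInitialized binds the health component's update and death events to the phase check and death handling.
; Dropping to the health threshold advances the blackboard CurrentPhase, spawns an explosion and teleports the boss to its phase-two location.
; Death enables mesh physics, unpossesses the AI controller and sets a timed despawn.
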(event `self.ReceiveBeginPlay`
  (`SkeletalMeshComponent.SetSkeletalMeshAsset` (`self.Weapon`) (`/Game/BLUEPRINTS/DataAssets/PDA_Weapons.WeaponComponent` (`self.EnemyWeapon`)))
  (`SceneComponent.K2_AttachToComponent` (`self.Weapon`) (`self.Mesh`) "hand_r" "KeepRelative" "KeepWorld" "KeepRelative" true))

(event `self.BossInitialized`
  (params (EnemyHealthComponent :type "HealthComponent Object Reference"))
  (`self.OnBossInitialized` EnemyHealthComponent)
  (add `HealthComponent.OnHealthUpdated` (`self.HealthComponent`) (delegate `CustomEvent_DamageReceived`))
  (add `HealthComponent.OnCharacterDeath` (`self.HealthComponent`) (delegate `CustomEvent_OnDeath`)))

(event `CustomEvent_OnDeath`
  (`self.OnDeath`))

(event `CustomEvent_DamageReceived`
  (params (NewHealth :type Integer) (OwnerComponentToUpdate :type "HealthComponent Object Reference"))
  (`self.CheckPhase`))

(event `/Game/BLUEPRINTS/Interfaces/BPI_DamageInterface.DamageEffects`
  (params (HitEffect :type "NiagaraSystem Object Reference"))
  (`NiagaraFunctionLibrary.SpawnSystemAttached` HitEffect (`self.HitTakenEffect`) "None" (0.0 0.0 0.0) (struct) "KeepRelativeOffset" true))

(fn `CheckPhase`
  (bind _returnvalue (`AIBlueprintHelperLibrary.GetBlackboard` null))
  (bind _healthcomponent (`self.HealthComponent`))
  (if (`HealthComponent.IsDead` (`self.HealthComponent`))
    _
    (elif (and (<= (`KismetMathLibrary.NormalizeToRange` (/ (`KismetMathLibrary.Conv_IntToDouble` (`HealthComponent.CurrentHealth` _healthcomponent)) (`KismetMathLibrary.Conv_IntToDouble` (`HealthComponent.MaxHealth` _healthcomponent))) 0.0 1.0) 0.6) (== (`BlackboardComponent.GetValueAsInt` _returnvalue "CurrentPhase") 1))
      (`BlackboardComponent.SetValueAsInt` _returnvalue "CurrentPhase" 2)
      (`self.EnterPhase2`))))

(fn `EnterPhase2`
  (`GameplayStatics.SpawnEmitterAtLocation` "/Game/StarterContent/Particles/P_Explosion.P_Explosion" (`self.K2_GetActorLocation`) (struct) (10.0 10.0 10.0))
  (`self.K2_SetActorTransform` (`self.Phase2SpawnLocation`) false true))

(fn `OnDeath`
  (bind _mesh (`self.Mesh`))
  (bind _asbp_boss_aicontroller (cast `/Game/BLUEPRINTS/BP_BossAIController` (`self.GetController`)))
  (`PrimitiveComponent.SetSimulatePhysics` _mesh true)
  (`PrimitiveComponent.SetCollisionEnabled` _mesh "QueryAndPhysics")
  (`Controller.UnPossess` _asbp_boss_aicontroller)
  (`self.SetLifeSpan` 30.0))

(fn `UserConstructionScript`)