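; BP_BossBeamShot is a short-lived boss beam attack that damages the player after a brief telegraph.
; InitializeBeam applies a dynamic material and starts a timer, using a while loop on its elapsed time to set beam opacity.
; When the timer fires, it hides the beam, activates BeamEffect and sphere-traces from BeamStart to BeamEnd.
; A blocking hit on BP_ThirdPersonCharacter deals fixed damage through its HealthComponent.
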(event `self.ReceiveBeginPlay`
  (`self.SetLifeSpan` 2.0))

(event `self.InitializeBeam`
  (params (StartLocation :type "Vector Structure") (EndLocation :type "Vector Structure"))
  (bind _returnvalue (`PrimitiveComponent.CreateDynamicMaterialInstance` (`self.Beam`) 0 "/Game/MATERIALS/MI_BeamShot.MI_BeamShot" "None"))
  (bind _output_get (set `self.MaterialToChange` _returnvalue))
  (`PrimitiveComponent.SetMaterial` (`self.Beam`) 0 _output_get)
  (bind _returnvalue_2 (`KismetSystemLibrary.K2_SetTimerDelegate` (delegate `CustomEvent_ApplyDamage`) 0.75))
  (bind _output_get_2 (set `self.OpacityTimer` _returnvalue_2))
  (while (`KismetSystemLibrary.K2_IsTimerActiveHandle` _output_get_2)
    (`MeshComponent.SetScalarParameterValueOnMaterials` (`self.Beam`) "Opacity" (`KismetSystemLibrary.K2_GetTimerElapsedTimeHandle` _output_get_2))))

(event `CustomEvent_ApplyDamage`
  (`SceneComponent.SetVisibility` (`self.Beam`) false false)
  (bind _outhit (`KismetSystemLibrary.SphereTraceSingle` (`SceneComponent.K2_GetComponentLocation` (`self.BeamStart`)) (`SceneComponent.K2_GetComponentLocation` (`self.BeamEnd`)) 50.0 "TraceTypeQuery4"))
  (`ActorComponent.Activate` (`self.BeamEffect`) true)
  (bind (_bblockinghit _binitialoverlap _time _distance _location _impactpoint _normal _impactnormal _physmat _hitactor) (`GameplayStatics.BreakHitResult` _outhit))
  (if _bblockinghit
    (`/Engine/EditorBlueprintResources/StandardMacros.IsValid` _hitactor
      (:`Is Valid`
        (bind _asbp_third_person_character (cast `/Game/ThirdPerson/Blueprints/BP_ThirdPersonCharacter` _hitactor))
        (`HealthComponent.TakeDamage` (`AIProgrammingCharacter.HealthComponent` _asbp_third_person_character) 50)))))

(fn `UserConstructionScript`)