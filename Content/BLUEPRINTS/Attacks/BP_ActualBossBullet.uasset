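; BP_ActualBossBullet is a boss attack bullet that deals hitscan damage to the player character.
; On BeginPlay it line-traces 5000 units forward from its own location.
; A third-person character hit takes damage through its HealthComponent and receives a hit-effect message.
; The bullet sets a short lifespan after hitting any valid actor, but sets none on a miss.
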(event `self.ReceiveBeginPlay`
  (bind _returnvalue (`self.K2_GetActorLocation`))
  (bind _outhit (`KismetSystemLibrary.LineTraceSingle` _returnvalue (+ _returnvalue (* (`self.GetActorForwardVector`) 5000.0)) "TraceTypeQuery5"))
  (bind (_bblockinghit _binitialoverlap _time _distance _location _impactpoint _normal _impactnormal _physmat _hitactor) (`GameplayStatics.BreakHitResult` _outhit))
  (if _bblockinghit
    (`/Engine/EditorBlueprintResources/StandardMacros.IsValid` _hitactor
      (:`Is Valid`
        (bind _asbp_third_person_character (cast `/Game/ThirdPerson/Blueprints/BP_ThirdPersonCharacter` _hitactor)
          (:`then`
            (`HealthComponent.TakeDamage` (`AIProgrammingCharacter.HealthComponent` _asbp_third_person_character) (`self.Damage`))
            (message `/Game/BLUEPRINTS/Interfaces/BPI_DamageInterface.DamageEffects` _asbp_third_person_character (`self.HitEffect`))
            (`self.SetLifeSpan` 0.2))
          (:`CastFailed`
            (`self.SetLifeSpan` 0.2)))))))

(fn `UserConstructionScript`)